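; Base interactable door that swings open away from the player and can be Opened (usable), Blocked or Locked.
; A timeline rotates the mesh yaw, with a dot product against the frame choosing the swing's sign.
; Optional auto-close runs on a timer, which an overlap count on the Inside volume is meant to pause and resume.
; Zap opens usable doors, or unlocks and opens locked ones with auto-close disabled.
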(event `/Game/Door/Interfaces/BPI_InteractBis.InteractBis`
  ;[0 0 0] OldSystem
  (switch `/Game/Door/Enum/Door_State` (`self.State`)
    (:`NewEnumerator0`
      (`self.BlockDoor`))
    (:`NewEnumerator2`
      (`self.UnBlockDoor`))))

(event `/Game/Door/Interfaces/BPI_Interact.Interact`
  (params (Investigator :type "Character Object Reference"))
  ;[0 0 0] OldSystem
)

(event `self.Interactable.On Interact`
  (params (Player :type "Pawn Object Reference"))
  (switch `/Game/Door/Enum/Door_State` (`self.State`)
    (:`NewEnumerator0`
      (if (`self.IsOppened`)
        (`self.CloseDoor`)
        (else
          (`self.SetOpenValue` Player)
          (`self.OpenDoor`))))))

(event `OpenDoor`
  ;[1 1 1] DoorOpen/Close
  (set `self.IsOppened` true)
  (bind (_direction _doorrotation) (`Timeline|Timeline_DoorAnimation` :!label _label)
    (:`Update`
      (`SceneComponent.K2_SetRelativeRotation` (`self.DoorMesh`) (`KismetMathLibrary.MakeRotator` 0.0 0.0 (`KismetMathLibrary.Lerp` 0.0 (`self.OpenAmount`) _doorrotation)) false false))
    (:`Finished`
      (if (`self.AutoClose?`)
        (bind _returnvalue (`KismetSystemLibrary.K2_SetTimerDelegate` (`|CreateDelegate` :!event `CloseDoor`) (`self.CloseDelay`)))
        (set `self.CloseTimer` _returnvalue)))))

(event `CloseDoor`
  ;[1 1 1] DoorOpen/Close
  (set `self.IsOppened` false)
  (goto _label :!via `Reverse`))

(event `self.Inside.OnComponentBeginOverlap`
  (params (OverlappedComponent :type "PrimitiveComponent Object Reference") (OtherActor :type "Actor Object Reference") (OtherComp :type "PrimitiveComponent Object Reference") (OtherBodyIndex :type Integer) (bFromSweep :type Boolean) (SweepResult :type "HitResult Structure (by ref)"))
  ;[1 1 1] CheckOverlappingInfo
  (`/Engine/EditorBlueprintResources/StandardMacros.IncrementInt` (`self.BlockedBySmth`)
    (:`  `
      (`self.ToggleDoorCloseTimer` true))))

(event `self.Inside.OnComponentEndOverlap`
  (params (OverlappedComponent :type "PrimitiveComponent Object Reference") (OtherActor :type "Actor Object Reference") (OtherComp :type "PrimitiveComponent Object Reference") (OtherBodyIndex :type Integer))
  ;[1 1 1] CheckOverlappingInfo
  (bind _result (`/Engine/EditorBlueprintResources/StandardMacros.DecrementInt` (`self.BlockedBySmth`))
    (:`  `
      (if (and (<= _result 0) (`self.IsOppened`) (`self.AutoClose?`))
        (`self.ToggleDoorCloseTimer` false)))))

(event `self.ReceiveBeginPlay`
  ;[1 1 1] CheckOverlappingInfo
  (set `self.BlockedBySmth` (`KismetArrayLibrary.Array_Length` (`PrimitiveComponent.GetOverlappingActors` (`self.Inside`) "/Script/Engine.Character"))))

(event `BlockDoor`
  (set `self.State` "NewEnumerator2"))

(event `LockDoor`
  (set `self.State` "NewEnumerator1"))

(event `UnBlockDoor`
  (set `self.State` "NewEnumerator0" :!label _label_2))

(event `UnLockDoor`
  (goto _label_2))

(event `/Game/Door/Interfaces/BPI_Electricity.Zap`
  (switch `/Game/Door/Enum/Door_State` (`self.State`)
    (:`NewEnumerator0`
      (if (not (`self.IsOppened`))
        (`self.OpenDoor` :!label _label_3)))
    (:`NewEnumerator1`
      (`self.UnLockDoor`)
      (set `self.AutoClose?` false)
      (goto _label_3))))

(fn `CanInteract`
  (params (Investigator :type "Character Object Reference"))
  (returns (Value :type Boolean))
  (return false))

(fn `CanInteractBis`
  (returns (Value :type Boolean))
  (return false))

(fn `Is Interactor in Front`
  (params (Actor :type "Actor Object Reference"))
  (returns (ReturnValue :type Boolean))
  (return (< (`KismetMathLibrary.Dot_VectorVector` (`self.GetActorForwardVector` Actor) (`SceneComponent.GetForwardVector` (`self.DoorFrameMesh`))) 0.0)))

(fn `IsDoorBlockedBySomthing`
  (returns (Return :type Boolean))
  (return (> (`self.BlockedBySmth`) 0)))

(fn `SetOpenValue`
  (params (Actor :type "Actor Object Reference"))
  (bind _returnvalue (> (`self.OpenAmount`) 0.0))
  (if (`self.Is Interactor in Front` Actor)
    (if _returnvalue
      (`/Engine/EditorBlueprintResources/StandardMacros.NegateFloat` (`self.OpenAmount`) :!label _label
        (:`  `
          (return))))
    (elif (not _returnvalue)
      (goto _label))))

(fn `ToggleDoorCloseTimer`
  (params (Pause :type Boolean))
  (bind _returnvalue (`KismetSystemLibrary.K2_IsTimerPausedHandle` (`self.CloseTimer`)))
  (if (`KismetSystemLibrary.K2_TimerExistsHandle` (`self.CloseTimer`))
    (if Pause
      (if _returnvalue
        (`KismetSystemLibrary.K2_PauseTimerHandle` (`self.CloseTimer`)))
      (elif (not _returnvalue)
        (`KismetSystemLibrary.K2_UnPauseTimerHandle` (`self.CloseTimer`)))))
  (return))

(fn `UserConstructionScript`)